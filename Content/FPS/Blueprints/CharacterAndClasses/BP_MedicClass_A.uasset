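; BP_MedicClass_A is the medic character class, whose ThrowItem event requests a server spawn of a BP_Medkit.
; CanUseAbility passes only when shooting, grenade and skill flags allow it and the character is not aiming, dead, busy or falling.
; Equip and unequip functions play first-person montages, delaying weapon reveal briefly to avoid a misplaced frame and hiding the weapon on unequip blend-out.
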(event `/Game/FPS/Blueprints/Interfaces/iPawnActions.ThrowItem`
  (`self.Server_SpawnMedKit` "/Game/FPS/Blueprints/Medkit/BP_Medkit.BP_Medkit_C"))

(fn `UserConstructionScript`
  (`parent.UserConstructionScript`))