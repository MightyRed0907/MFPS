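; Behavior tree task that lets an AI-controlled player character interact with nearby bombs in the Rush game mode.
; For a living pawn, it loops over the bomb references in the Rush game state and calls the AI interact function on each valid bomb within a short radius.
; It then clears the interact blackboard flag and finishes successfully, but never finishes if the pawn is dead or a cast fails.
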(event `self.ReceiveExecuteAI`
  (params (OwnerController :type "AIController Object Reference") (ControlledPawn :type "Pawn Object Reference"))
  ;[1 1 1] Interact with objective
  (bind _asbp_player_character (cast `/Game/FPS/Blueprints/CharacterAndClasses/BP_PlayerCharacter` ControlledPawn))
  (if (not (`/Game/FPS/Blueprints/CharacterAndClasses/BP_BaseCharacter.bDead` _asbp_player_character))
    (bind _asbp_rush_gs (cast `/Game/FPS/Blueprints/GameModes/Rush/BP_Rush_GS` (`GameplayStatics.GetGameState`)))
    (for _array_element (`/Game/FPS/Blueprints/GameModes/Rush/BP_Rush_GS.BombRef` _asbp_rush_gs)
      (`/Engine/EditorBlueprintResources/StandardMacros.IsValid` _array_element
        (:`Is Valid`
          (if (<= (`KismetMathLibrary.VSize` (- (`Actor.K2_GetActorLocation` _array_element) (`Actor.K2_GetActorLocation` ControlledPawn))) 500.0)
            (`/Game/FPS/Blueprints/GameObjectives/RushObjective/BP_RushObjective.AI_BombInteract` _array_element _asbp_player_character)))))
    (`BTFunctionLibrary.SetBlackboardValueAsBool` (`self.InteractBombKey`))
    (`self.FinishExecute` true)))