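; Behavior tree service that supplies AI with the location of a random living player.
; Each tick, GetPlayers gathers player character pawns from the GameState's PlayerArray, and FindPlayers drops dead ones and the controlled pawn.
; A random entry's location is written to the Vectorkey blackboard key as a position snapshot.
; The random index is rolled separately for the validity check and the write, so they can hit different players.
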(event `self.ReceiveTickAI`
  (params (OwnerController :type "AIController Object Reference") (ControlledPawn :type "Pawn Object Reference") (DeltaSeconds :type "Float (single-precision)"))
  (bind _newparam (`self.GetPlayers`))
  (bind _enemies (`self.FindPlayers` ControlledPawn _newparam))
  (if (`KismetArrayLibrary.Array_IsValidIndex` _enemies)
    (bind _output (`|GetArrayItem` _enemies (`KismetMathLibrary.RandomIntegerInRange` 0 (`KismetArrayLibrary.Array_LastIndex` _enemies))))
    (`/Engine/EditorBlueprintResources/StandardMacros.IsValid` _output
      (:`Is Valid`
        (`BTFunctionLibrary.SetBlackboardValueAsVector` (`self.Vectorkey`) (`Actor.K2_GetActorLocation` _output))))))

(fn `FindPlayers`
  (params (SelfPawn :type "Pawn Object Reference") (PossibleEnemies :type "Array of /Game/FPS/Blueprints/CharacterAndClasses/BP_PlayerCharacter Object Reference"))
  (returns (Enemies :type "Array of /Game/FPS/Blueprints/CharacterAndClasses/BP_PlayerCharacter Object Reference"))
  (locals (EnemiesArray :type "Array of /Game/FPS/Blueprints/CharacterAndClasses/BP_PlayerCharacter Object Reference"))
  (`KismetArrayLibrary.Array_Clear` (`local.EnemiesArray`))
  (for _array_element PossibleEnemies
    (if (and (!= _array_element (cast `/Game/FPS/Blueprints/CharacterAndClasses/BP_PlayerCharacter` SelfPawn :!pure true)) (not (`/Game/FPS/Blueprints/CharacterAndClasses/BP_BaseCharacter.bDead` _array_element)))
      (`KismetArrayLibrary.Array_AddUnique` (`local.EnemiesArray`) _array_element)))
  (return (`local.EnemiesArray`)))

(fn `GetPlayers`
  (returns (NewParam :type "Array of /Game/FPS/Blueprints/CharacterAndClasses/BP_PlayerCharacter Object Reference"))
  (locals (Players :type "Array of /Game/FPS/Blueprints/CharacterAndClasses/BP_PlayerCharacter Object Reference"))
  (for _array_element (`GameStateBase.PlayerArray` (`GameplayStatics.GetGameState`))
    (bind _asbp_player_character (cast `/Game/FPS/Blueprints/CharacterAndClasses/BP_PlayerCharacter` (`PlayerState.PawnPrivate` _array_element)))
    (`KismetArrayLibrary.Array_AddUnique` (`local.Players`) _asbp_player_character))
  (return (`local.Players`)))