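; Blueprint function library that gives access to the HUD_CompShooter shooter HUD and its events.
; Getters resolve the HUD from the first player, a player index, a PlayerController or a Controller by casting the controller's HUD, most printing an error on failure.
; Helpers bind delegates to tutorial-message confirmation, progress bar completion and timer completion, with unbinding offered only for the timer.
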(fn `BindLastMainTutorialMessageConfirmed`
  (params (PlayerController :type "PlayerController Object Reference") (OnTutorialMessageConfirmed :type "Delegate (by ref)"))
  (bind _ashud_comp_shooter (cast `/Game/CompShooterHUD/Blueprints/HUD_CompShooter` (`PlayerController.GetHUD` PlayerController))
    (:`then`
      (add `/Game/CompShooterHUD/Blueprints/HUD_CompShooter.MainTutorialMessageConfirmed` _ashud_comp_shooter OnTutorialMessageConfirmed))
    (:`CastFailed`
      (`KismetSystemLibrary.PrintString` null "Cast to HUD failed. Please check your PC Reference!" true true (struct :`G` 0.66 :`B` 1.0 :`A` 1.0) 4.0))))

(fn `BindOnProgressBarCompleted`
  (params (`Player Controller` :type "PlayerController Object Reference") (OnProgressBarCompleted :type "Delegate (by ref)"))
  (bind _ashud_comp_shooter (cast `/Game/CompShooterHUD/Blueprints/HUD_CompShooter` (`PlayerController.GetHUD` `Player Controller`))
    (:`then`
      (add `/Game/CompShooterHUD/Blueprints/HUD_CompShooter.OnProgressBarCompleted` _ashud_comp_shooter OnProgressBarCompleted))
    (:`CastFailed`
      (`KismetSystemLibrary.PrintString` null "Cast to HUD failed. Please check your PC Reference!" true true (struct :`G` 0.66 :`B` 1.0 :`A` 1.0) 4.0))))

(fn `BindOnTimerFinished`
  (params (PlayerIndex :type Integer) (Event :type "Delegate (by ref)"))
  (bind _ashud_comp_shooter (`self.GetShooterHud` PlayerIndex))
  (`/Engine/EditorBlueprintResources/StandardMacros.IsValid` _ashud_comp_shooter
    (:`Is Valid`
      (add `/Game/CompShooterHUD/Blueprints/HUD_CompShooter.OnTimerCompleted` _ashud_comp_shooter Event)
      (return))
    (:`Is Not Valid`
      (return))))

(fn `GetShooterHud`
  (params (PlayerIndex :type Integer))
  (returns (`AsHUD Comp Shooter` :type "/Game/CompShooterHUD/Blueprints/HUD_CompShooter Object Reference"))
  (bind _ashud_comp_shooter (cast `/Game/CompShooterHUD/Blueprints/HUD_CompShooter` (`PlayerController.GetHUD` (`GameplayStatics.GetPlayerController` null PlayerIndex))))
  (return _ashud_comp_shooter))

(fn `GetShooterHudManager`
  (returns (ShooterHudManager :type "/Game/CompShooterHUD/Blueprints/Interfaces/I_ShooterHudManager Interface"))
  (bind _ashud_comp_shooter (cast `/Game/CompShooterHUD/Blueprints/HUD_CompShooter` (`PlayerController.GetHUD` (`GameplayStatics.GetPlayerController` null)))
    (:`then`
      (return _ashud_comp_shooter))
    (:`CastFailed`
      (`KismetSystemLibrary.PrintString` null "FL_ShooterHUD: Cast to HUD_CompShooter failed!" true true (struct :`R` 1.0 :`G` 0.230857 :`A` 1.0) 10.0))))

(fn `GetShooterHudManagerFromController`
  (params (Controller :type "Controller Object Reference"))
  (returns (ShooterHudManager :type "/Game/CompShooterHUD/Blueprints/Interfaces/I_ShooterHudManager Interface"))
  (bind _asplayer_controller (cast `PlayerController` Controller)
    (:`then`
      (bind _ashud_comp_shooter (cast `/Game/CompShooterHUD/Blueprints/HUD_CompShooter` (`PlayerController.GetHUD` _asplayer_controller))
        (:`then`
          (return _ashud_comp_shooter))
        (:`CastFailed`
          (`KismetSystemLibrary.PrintString` null "FL_ShooterHUD: Cast to HUD_CompShooter failed!" true true (struct :`R` 1.0 :`G` 0.230857 :`A` 1.0) 10.0))))
    (:`CastFailed`
      (`KismetSystemLibrary.PrintString` null "FL_ShooterHUD: Cast to PlayerController Instance failed!" true true (struct :`R` 1.0 :`G` 0.230857 :`A` 1.0) 10.0))))

(fn `GetShooterHudManagerFromPlayer`
  (params (PlayerController :type "PlayerController Object Reference"))
  (returns (ShooterHudManager :type "/Game/CompShooterHUD/Blueprints/Interfaces/I_ShooterHudManager Interface"))
  (bind _ashud_comp_shooter (cast `/Game/CompShooterHUD/Blueprints/HUD_CompShooter` (`PlayerController.GetHUD` PlayerController))
    (:`then`
      (return _ashud_comp_shooter))
    (:`CastFailed`
      (`KismetSystemLibrary.PrintString` null "FL_ShooterHUD: Cast to HUD_CompShooter failed!" true true (struct :`R` 1.0 :`G` 0.230857 :`A` 1.0) 10.0))))

(fn `UnbindOnTimerFinished`
  (params (PlayerIndex :type Integer) (Event :type "Delegate (by ref)"))
  (bind _ashud_comp_shooter (`self.GetShooterHud` PlayerIndex))
  (`/Engine/EditorBlueprintResources/StandardMacros.IsValid` _ashud_comp_shooter
    (:`Is Valid`
      (remove `/Game/CompShooterHUD/Blueprints/HUD_CompShooter.OnTimerCompleted` _ashud_comp_shooter Event)
      (return))
    (:`Is Not Valid`
      (return))))