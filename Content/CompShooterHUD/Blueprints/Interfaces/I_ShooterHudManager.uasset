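; Blueprint interface for the shooter HUD manager, defining the calls that gameplay code can use to drive the on-screen HUD.
; It covers crosshair, zoom and recoil, hit and damage feedback, kill feed, medals, achievements, tutorial messages and screen effects.
; It also declares health, armor, weapon and ammo bars, action slots, team kill counts and a match timer, with getters for current values.
; It holds only signatures, with no logic of its own.
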(fn `AddAchievement`
  (params (Display_Time :type "Float (double-precision)") (Achievement_Widget :type "UserWidget Class Reference") (Anim_Color :type "LinearColor Structure") (Background_Color :type "LinearColor Structure") (Achievement_Text :type Text) (Text_Color :type "LinearColor Structure")))

(fn `AddArmorBar`
  (params (ProgressBar_Color :type "LinearColor Structure") (Progress_Color :type "LinearColor Structure") (Text_Color :type "LinearColor Structure") (Frame_Color :type "LinearColor Structure") (Damage_Color :type "LinearColor Structure") (Armor_Color :type "LinearColor Structure") (Armor_Icon :type "UserWidget Class Reference") (MaxArmorSensitive :type Boolean)))

(fn `AddDamageFeedback`
  (params (FeedbackColor :type "LinearColor Structure")))

(fn `AddDamageIndicator`
  (params (Color :type "LinearColor Structure") (Display_Time :type "Float (double-precision)") (bViewportSensitive :type Boolean) (OwningCamera :type "CameraComponent Object Reference") (Instigator :type "Actor Object Reference")))

(fn `AddExtraTime`
  (params (XtraSeconds :type Integer) (EmptyColor :type "LinearColor Structure") (FillColor :type "LinearColor Structure") (TextColor :type "LinearColor Structure")))

(fn `AddHealthBar`
  (params (ProgressBar_Color :type "LinearColor Structure") (Progress_Color :type "LinearColor Structure") (Text_Color :type "LinearColor Structure") (Frame_Color :type "LinearColor Structure") (Damage_Color :type "LinearColor Structure") (Health_Color :type "LinearColor Structure") (Icon :type "UserWidget Class Reference") (IsMaxHealthSensitive :type Boolean) (bUseLowDamagePostProcess :type Boolean)))

(fn `AddIntermediatePoints`
  (params (DisplayTime :type "Float (double-precision)") (Entry :type "/Game/CompShooterHUD/Blueprints/Structs/S_IntPoints Structure") (SummaryTextColor :type "LinearColor Structure")))

(fn `AddKillMessage1`
  (params (Display_Time :type "Float (double-precision)") (Head_Color :type "LinearColor Structure") (Child_Color :type "LinearColor Structure") (HeadText_Bold :type Text) (HeadText_Regular :type Text) (ChildText_Bold :type Text) (ChildText_Regular :type Text) (Causer_Icon :type "Object Object Reference") (Causer_IconColor :type "LinearColor Structure")))

(fn `AddKillMessage2`
  (params (Head_Color :type "LinearColor Structure") (Child_Color :type "LinearColor Structure") (Display_Time :type "Float (double-precision)") (Head_Text_Bold :type Text) (InstigatorName :type Text) (Causer_Icon :type "Object Object Reference") (Causer_Icon_Color :type "LinearColor Structure") (InstigatorHealth :type Integer) (InstigatorShield :type Integer) (InstigatorArmor :type Integer)))

(fn `AddMainTutorialMessage`
  (params (`BlurBackground?` :type Boolean) (UseTutorialVisual :type Boolean) (Tutorial_VisualInfo :type "/Game/CompShooterHUD/Blueprints/Structs/S_TutorialVideoInfo Structure") (UseHeadlineIcon :type Boolean) (Headline_IconInfo :type "/Game/CompShooterHUD/Blueprints/Structs/S_IconInfo Structure") (MainTutorialInfo :type "/Game/CompShooterHUD/Blueprints/Structs/S_MainTutorialMessage Structure") (bUseCustomTextWidget :type Boolean) (CustomTextWidget :type "UserWidget Class Reference") (Background_Color :type "LinearColor Structure") (bUseButton :type Boolean) (ButtonText :type Text) (ButtonTextColor :type "LinearColor Structure") (ButtonIconInfo :type "/Game/CompShooterHUD/Blueprints/Structs/S_IconInfo Structure"))
  (return))

(fn `AddMedal`
  (params (DisplayTime :type "Float (double-precision)") (MedalWidget :type "UserWidget Class Reference") (Text :type Text) (Value :type Text) (TextColor :type "LinearColor Structure") (HighlightColor :type "LinearColor Structure")))

(fn `AddNewKillEntry`
  (params (KillCountEntryInfo :type "/Game/CompShooterHUD/Blueprints/Structs/S_KillCountEntry Structure")))

(fn `AddOrUpdateActionSlot`
  (params (E_Slot :type "/Game/CompShooterHUD/Blueprints/Enums/E_ActionSlots Enum" :default "NewEnumerator0") (Slot_KeyText :type Text) (Slot_KeyColor :type "LinearColor Structure") (Slot_Icon :type "Object Object Reference") (Slot_IconColor :type "LinearColor Structure") (Slot_FrameColor :type "LinearColor Structure") (Slot_FrameShineColor :type "LinearColor Structure")))

(fn `AddOrUpdateAmmoIcon`
  (params (Icon_Slot :type "/Game/CompShooterHUD/Blueprints/Enums/E_AmmoSlots Enum" :default "NewEnumerator0") (Slot_AnimColor :type "LinearColor Structure") (Slot_Icon :type "UserWidget Class Reference")))

(fn `AddOrUpdateCrosshair`
  (params (CrosshairType :type "/Game/CompShooterHUD/Blueprints/Enums/E_CrosshairType Enum" :default "NewEnumerator0") (CrosshairColor :type "LinearColor Structure") (CrosshairScale :type "Float (double-precision)" :default 1.0) (bUseMovementSensitivity :type Boolean) (MovementSensitivityCharacter :type "Character Object Reference")))

(fn `AddOrUpdateProgressBar`
  (params (ProgressBarType :type "/Game/CompShooterHUD/Blueprints/Enums/E_ProgressBars Enum" :default "NewEnumerator0") (ProgressType :type "/Game/CompShooterHUD/Blueprints/Enums/E_ProgressBarType Enum" :default "NewEnumerator0") (ProgressTime :type "Float (double-precision)") (ProgressValue :type "Float (double-precision)") (Empty_Color :type "LinearColor Structure") (Fill_Color :type "LinearColor Structure")))

(fn `AddOrUpdateTeamKillCount`
  (params (E_Team :type "/Game/CompShooterHUD/Blueprints/Enums/E_TeamCount Enum" :default "NewEnumerator0") (Team_Name :type Text) (Team_TextColor :type "LinearColor Structure") (Value_TextColor :type "LinearColor Structure") (Progress_FrameColor :type "LinearColor Structure") (Progress_Color :type "LinearColor Structure") (Border_Color :type "LinearColor Structure")))

(fn `AddOrUpdateZoom`
  (params (bZoomIn :type Boolean) (ZoomValueDegrees :type "Float (double-precision)") (PlayerCamera :type "CameraComponent Object Reference") (ScopeInfo :type "/Game/CompShooterHUD/Blueprints/Structs/S_ScopeInfo Structure")))

(fn `AddRecoil`)

(fn `AddWeaponBar`
  (params (Ammo_ValueColor :type "LinearColor Structure") (MaxAmmo_ValueColor :type "LinearColor Structure") (Frame_Color :type "LinearColor Structure") (ProgressColor :type "LinearColor Structure") (WeaponColor :type "LinearColor Structure") (ProgressImpactColor :type "LinearColor Structure")))

(fn `CreateTimer`
  (params (Minutes :type Integer) (Seconds :type Integer) (ETimerMode :type "/Game/CompShooterHUD/Blueprints/Enums/E_TimerMode Enum" :default "NewEnumerator0") (Color :type "LinearColor Structure")))

(fn `DisplayHitPoint`
  (params (HitLocation :type "Vector Structure") (PointsColor :type "LinearColor Structure") (PointsText :type Text)))

(fn `DisplayShooterHUD`
  (params (State :type "/Game/CompShooterHUD/Blueprints/Enums/E_DisplayStates Enum" :default "NewEnumerator0") (ZOrder :type Integer :default 1)))

(fn `DisplaySpecialHitPoint`
  (params (HitLocation :type "Vector Structure") (PointsColor :type "LinearColor Structure") (PointsText :type Text)))

(fn `GetCurrentAmmo`
  (returns (Ammo :type Integer))
  (return 0))

(fn `GetCurrentAmmoType`
  (returns (AmmoType :type "/Game/CompShooterHUD/Blueprints/Enums/E_AmmoType Enum"))
  (return "NewEnumerator0"))

(fn `GetCurrentArmor`
  (returns (ArmorValue :type Integer))
  (return 0))

(fn `GetCurrentHealth`
  (returns (HealthValue :type Integer))
  (return 0))

(fn `GetCurrentMaxAmmo`
  (returns (MaxAmmo :type Integer))
  (return 0))

(fn `GetCurrentMaxArmor`
  (returns (CurrentMaxArmor :type Integer))
  (return 0))

(fn `GetCurrentMaxHealth`
  (returns (CurrentMaxHealth :type Integer))
  (return 0))

(fn `GetCurrentStackSize`
  (returns (Stack_Size :type Integer))
  (return 0))

(fn `GetLastKillEntry`
  (returns (InstigatorName :type Text) (CauserIcon :type "Object Object Reference") (DamagedName :type Text))
  (return "" null ""))

(fn `GetTeamKillCountMaxValue`
  (params (E_Team :type "/Game/CompShooterHUD/Blueprints/Enums/E_TeamCount Enum" :default "NewEnumerator0"))
  (returns (TeamKillCountMaxValue :type Integer))
  (return 0))

(fn `GetTeamKillCountValue`
  (params (E_Team :type "/Game/CompShooterHUD/Blueprints/Enums/E_TeamCount Enum" :default "NewEnumerator0"))
  (returns (TeamKillCountValue :type Integer))
  (return 0))

(fn `GetTime`
  (returns (Minutes :type Integer) (Seconds :type Integer))
  (return 0 0))

(fn `HitIndicator`
  (params (IndicatorType :type "/Game/CompShooterHUD/Blueprints/Enums/E_HitIndicators Enum" :default "NewEnumerator0") (IndicatorColor :type "LinearColor Structure")))

(fn `PauseTimer`
  (params (`Pause/Unpause` :type Boolean)))

(fn `RemoveAchievement`)

(fn `RemoveActionSlot`
  (params (ActionSlot :type "/Game/CompShooterHUD/Blueprints/Enums/E_ActionSlots Enum" :default "NewEnumerator0")))

(fn `RemoveAllActionSlots`)

(fn `RemoveAllDamageIndicator`)

(fn `RemoveAmmo`
  (params (Ammo :type Integer)))

(fn `RemoveAmmoIcon`
  (params (IconSlot :type "/Game/CompShooterHUD/Blueprints/Enums/E_AmmoSlots Enum" :default "NewEnumerator0") (bRemoveAllIcons :type Boolean)))

(fn `RemoveArmor`
  (params (Damage_Value :type Integer) (bUsePostProcessFX :type Boolean)))

(fn `RemoveArmorBar`)

(fn `RemoveCrosshair`)

(fn `RemoveDamageFeedback`)

(fn `RemoveHealth`
  (params (DamageValue :type Integer) (bUsePostProcessFX :type Boolean)))

(fn `RemoveHealthBar`)

(fn `RemoveHitPoint`)

(fn `RemoveIntermediatePoints`)

(fn `RemoveKillEntrys`)

(fn `RemoveKillMessages`)

(fn `RemoveMainTutorialMessage`
  (return))

(fn `RemoveMaxAmmo`
  (params (MaxAmmo :type Integer)))

(fn `RemoveMedal`)

(fn `RemoveProgressBar`)

(fn `RemoveSpecialHitPoint`)

(fn `RemoveTeamKillCount`
  (params (E_Team :type "/Game/CompShooterHUD/Blueprints/Enums/E_TeamCount Enum" :default "NewEnumerator0")))

(fn `RemoveTeamKillCountMaxValue`
  (params (E_Team :type "/Game/CompShooterHUD/Blueprints/Enums/E_TeamCount Enum" :default "NewEnumerator0") (Value :type Integer) (ImpactColor :type "LinearColor Structure")))

(fn `RemoveTeamKillCountValue`
  (params (E_Team :type "/Game/CompShooterHUD/Blueprints/Enums/E_TeamCount Enum" :default "NewEnumerator0") (Value :type Integer) (Impact_Color :type "LinearColor Structure")))

(fn `RemoveTimer`)

(fn `RemoveWeaponBar`)

(fn `SlotImpact`
  (params (Slot :type "/Game/CompShooterHUD/Blueprints/Enums/E_ActionSlots Enum" :default "NewEnumerator0")))

(fn `StartTimer`)

(fn `UpdateAmmo`
  (params (Ammo :type Integer) (Update_Type :type "/Game/CompShooterHUD/Blueprints/Enums/E_UpdateTypes Enum" :default "NewEnumerator0")))

(fn `UpdateArmor`
  (params (Value :type Integer) (UpdateType :type "/Game/CompShooterHUD/Blueprints/Enums/E_UpdateTypes Enum" :default "NewEnumerator0") (bUsePostProcessFX :type Boolean)))

(fn `UpdateBlackscreen_CSHUD`
  (params (DisplayBlackscreen :type Boolean) (SlowFading :type Boolean)))

(fn `UpdateColorImpact_CSHUD`
  (params (Color :type "LinearColor Structure")))

(fn `UpdateDamageFX_CSHUD`
  (params (State :type "/Game/CompShooterHUD/Blueprints/Enums/E_CSH_DamageStates Enum" :default "NewEnumerator0") (bDisplayDamage :type Boolean)))

(fn `UpdateHealth`
  (params (Value :type Integer) (UpdateType :type "/Game/CompShooterHUD/Blueprints/Enums/E_UpdateTypes Enum" :default "NewEnumerator0") (bUsePostProcessFX :type Boolean)))

(fn `UpdateMaxAmmo`
  (params (MaxAmmo :type Integer) (Update_Type :type "/Game/CompShooterHUD/Blueprints/Enums/E_UpdateTypes Enum" :default "NewEnumerator0")))

(fn `UpdateMaxArmor`
  (params (Max_Armor :type Integer)))

(fn `UpdateMaxHealth`
  (params (Max_Health_Value :type Integer)))

(fn `UpdateTeamKillCountMaxValue`
  (params (E_Team :type "/Game/CompShooterHUD/Blueprints/Enums/E_TeamCount Enum" :default "NewEnumerator0") (Value :type Integer) (Update_Type :type "/Game/CompShooterHUD/Blueprints/Enums/E_UpdateTypes Enum" :default "NewEnumerator0")))

(fn `UpdateTeamKillCountValue`
  (params (E_Team :type "/Game/CompShooterHUD/Blueprints/Enums/E_TeamCount Enum" :default "NewEnumerator0") (Value :type Integer) (Update_Type :type "/Game/CompShooterHUD/Blueprints/Enums/E_UpdateTypes Enum" :default "NewEnumerator0")))

(fn `UpdateWeaponBar`
  (params (Weapon_Icon :type "Object Object Reference") (Weapon_Name :type String) (Ammo_Type :type "/Game/CompShooterHUD/Blueprints/Enums/E_AmmoType Enum" :default "NewEnumerator0") (Stack_Size :type Integer)))